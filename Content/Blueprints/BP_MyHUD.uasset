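; BP_MyHUD keeps the game score and shows it on screen through a WBP_Sample widget.
; On BeginPlay it creates the widget, stores it in UpdataScore, pushes the current Score and adds it to the viewport.
; The AccGameScore event increments Score and calls the widget's UpdateScore.
; ActorBeginOverlap only re-sends the unchanged Score to the widget.
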(event `self.ReceiveBeginPlay`
  (bind _returnvalue (`|CreateWidget` "/Game/WBP_Sample.WBP_Sample_C"))
  (bind _output_get (set `self.Updata Score` _returnvalue))
  (`/Game/WBP_Sample.Update Score` _output_get (`self.Score`))
  (`UserWidget.AddToViewport` _returnvalue 0))

(event `self.ReceiveActorBeginOverlap`
  (params (OtherActor :type "Actor Object Reference"))
  (`/Game/WBP_Sample.Update Score` (`self.Updata Score`) (`self.Score`)))

(event `Acc GameScore`
  (`/Engine/EditorBlueprintResources/StandardMacros.IncrementInt` (`self.Score`)
    (:`  `
      (`/Game/WBP_Sample.Update Score` (`self.Updata Score`) (`self.Score`)))))

(fn `UserConstructionScript`)