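; BP_MYPC is a player controller that drives a BP_BasePawn and lets the player switch to another pawn.
; On possession it caches the pawn, whose multipliers scale yaw-relative movement and jumping.
; Enhanced Input handles look and movement, while jump directly offsets the pawn along its up vector on both press and release, without sweeping.
; Completing the interact input possesses the cached pawn's overlapping pawn.
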(event `self.ReceivePossess`
  (params (PossessedPawn :type "Pawn Object Reference"))
  (bind _asbp_base_pawn (cast `/Game/BP_BasePawn` PossessedPawn)
    (:`then`
      (set `self.PossessedBasePawn` _asbp_base_pawn))
    (:`CastFailed`
      (set `self.PossessedBasePawn` _asbp_base_pawn))))

(event `EnhancedInput|/Game/input/Action/IA_Look`
  (params (ActionValue :type "Vector2D Structure") (ElapsedSeconds :type "Float (double-precision)") (TriggeredSeconds :type "Float (double-precision)") (InputAction :type "InputAction Object Reference" :default "/Game/input/Action/IA_Look.IA_Look"))
  (bind _returnvalue (`self.K2_GetPawn`))
  (:`Triggered`
    (`Pawn.AddControllerYawInput` _returnvalue ActionValue_X)
    (`Pawn.AddControllerPitchInput` _returnvalue ActionValue_Y)))

(event `EnhancedInput|/Game/input/Action/IA_MOve`
  (params (ActionValue :type "Vector2D Structure") (ElapsedSeconds :type "Float (double-precision)") (TriggeredSeconds :type "Float (double-precision)") (InputAction :type "InputAction Object Reference" :default "/Game/input/Action/IA_MOve.IA_MOve"))
  (bind (_returnvalue_roll _returnvalue_pitch _returnvalue_yaw) (`KismetMathLibrary.BreakRotator` (`self.GetControlRotation`)))
  (bind (_returnvalue_roll_2 _returnvalue_pitch_2 _returnvalue_yaw_2) (`KismetMathLibrary.BreakRotator` (`self.GetControlRotation`)))
  (bind _returnvalue (`self.K2_GetPawn`))
  (bind _possessedbasepawn (`self.PossessedBasePawn`))
  (:`Triggered`
    (`|ExecutionSequence`
      (:`then_0`
        (`Pawn.AddMovementInput` _returnvalue (* (* ActionValue_X (`/Game/BP_BasePawn.MoveMultiplier` _possessedbasepawn)) (`KismetMathLibrary.GetRightVector` (`KismetMathLibrary.MakeRotator` _returnvalue_roll_2 0.0 _returnvalue_yaw_2))) 1.0 false))
      (:`then_1`
        (`Pawn.AddMovementInput` _returnvalue (* (* ActionValue_Y (`/Game/BP_BasePawn.MoveMultiplier` _possessedbasepawn)) (`KismetMathLibrary.GetForwardVector` (`KismetMathLibrary.MakeRotator` 0.0 0.0 _returnvalue_yaw))) 1.0 false)))))

(event `EnhancedInput|/Game/input/Action/IA_JUMP`
  (params (ActionValue :type Boolean) (ElapsedSeconds :type "Float (double-precision)") (TriggeredSeconds :type "Float (double-precision)") (InputAction :type "InputAction Object Reference" :default "/Game/input/Action/IA_JUMP.IA_JUMP"))
  (bind _returnvalue (`self.K2_GetPawn`))
  (bind _jumpmultiplier (`/Game/BP_BasePawn.JumpMultiplier` (`self.PossessedBasePawn`)))
  (bind _returnvalue_2 (* _jumpmultiplier (`SceneComponent.GetUpVector` (`Actor.RootComponent` (`self.K2_GetPawn`)))))
  (:`Started`
    (`self.K2_AddActorWorldOffset` _returnvalue _returnvalue_2 false false))
  (:`Completed`
    (`self.K2_AddActorWorldOffset` _returnvalue (* _returnvalue_2 _jumpmultiplier) false false)))

(event `EnhancedInput|/Game/input/Action/IA_Interalt`
  (params (ActionValue :type Boolean) (ElapsedSeconds :type "Float (double-precision)") (TriggeredSeconds :type "Float (double-precision)") (InputAction :type "InputAction Object Reference" :default "/Game/input/Action/IA_Interalt.IA_Interalt"))
  (bind _possessedbasepawn (`self.PossessedBasePawn`))
  (:`Completed`
    (`/Engine/EditorBlueprintResources/StandardMacros.IsValid` _possessedbasepawn
      (:`Is Valid`
        (`self.Possess` (`/Game/BP_BasePawn.OverlappintPawn` _possessedbasepawn))))))

(fn `UserConstructionScript`)