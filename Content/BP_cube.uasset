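; BP_cube is an actor that slides back and forth along world X around its starting position while ISMovingActor is true.
; The first Tick caches the starting X through a DoOnce.
; Each Tick steps by XMulitp, not scaled by delta time, and flips IsLoc to reverse when the next step would pass AbsoluteMaxX either side of the start.
; WBP_Sample creation and an alternative move are unconnected leftover nodes.
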(event `self.ReceiveBeginPlay`
  ;[1 1 1] Widget
)

(event `self.ReceiveTick`
  (params (DeltaSeconds :type "Float (single-precision)"))
  (bind _x_mulitp (`self.x mulitp`))
  (bind _absolute_max_x (`self.absolute max X`))
  (bind _returnvalue (+ (`self.inital X`) (select `bool` (`self.Is Loc`) :`false` (* _absolute_max_x -1.0) :`true` _absolute_max_x)))
  (bind _returnvalue_2 (+ (select `bool` (`self.Is Loc`) :`false` (* _x_mulitp -1.0) :`true` _x_mulitp) (.x (`self.K2_GetActorLocation`))))
  (`|ExecutionSequence`
    (:`then_0`
      ;[1 1 1] 초기 좌표값 설정
      (`/Engine/EditorBlueprintResources/StandardMacros.DoOnce` false
        (:`Completed`
          (set `self.inital X` (.x (`self.K2_GetActorLocation`))))))
    (:`then_1`
      (if (`self.IS Moving Actor`)
        (if (select `bool` (`self.Is Loc`) :`false` (< _returnvalue_2 _returnvalue) :`true` (> _returnvalue_2 _returnvalue))
          (set `self.Is Loc` (not (`self.Is Loc`)))
          (else
            (`self.K2_SetActorLocation` (`KismetMathLibrary.MakeVector` _returnvalue_2 (.y (`self.K2_GetActorLocation`)) (.z (`self.K2_GetActorLocation`))))))))))

(fn `UserConstructionScript`)