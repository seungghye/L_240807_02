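; Game instance Blueprint that handles level changes with a fade to white.
; OpenNewLevel starts a white camera fade on the first player, waits FadeDuration, then opens the given level by object reference.
; Unconnected nodes for stream-loading a level and fading back from white never run.
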(event `OpenNewLevel`
  (params (Level :type "World Soft Object Reference"))
  (`|ExecutionSequence`
    (:`then_0`
      (`PlayerCameraManager.StartCameraFade` (`PlayerController.PlayerCameraManager` (`GameplayStatics.GetPlayerController` 0)) 0.0 1.0 (`self.FadeDuration`) (struct :`R` 1.0 :`G` 1.0 :`B` 1.0 :`A` 1.0) false false))
    (:`then_1`
      (`KismetSystemLibrary.Delay` (`self.FadeDuration`))
      (`GameplayStatics.OpenLevelBySoftObjectPtr` Level))))